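; BP_EditorActor is an editor actor Blueprint that can tint its mesh to show valid or invalid state.
; Construction creates a dynamic M_Validation instance on VisualMesh's first material slot and hides it with zero opacity.
; SetValidationMat makes it half-opaque green or red by validity, and ClearValidationMat hides it again.
; Despite the OverlayDynMat name, the SetOverlayMaterial call is unconnected, and the event graph is empty.
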(event EventBeginPlay)

(event Collision|EventActorBeginOverlap
  (params (OtherActor :type Actor%20Object%20Reference)))

(event EventTick
  (params (DeltaSeconds :type Float%20%28single-precision%29)))

(fn ConstructionScript
  (bind _returnvalue (Rendering|Material|CreateDynamicMaterialInstance (Variables|Default|GetVisualMesh) 0 "/Game/EditorUI/Materials/M_Validation.M_Validation" "None" :!class /Script/Engine.PrimitiveComponent))
  (bind _output_get (Variables|Default|SetOverlayDynMat _returnvalue))
  (Rendering|Material|SetScalarParameterValue _output_get "Opacity" 0.0 :!class /Script/Engine.MaterialInstanceDynamic))

(fn SetValidationMat
  (params (Valid :type Boolean))
  (bind _overlaydynmat (Variables|Default|GetOverlayDynMat))
  (Rendering|Material|SetScalarParameterValue (Variables|Default|GetOverlayDynMat) "Opacity" 0.5 :!class /Script/Engine.MaterialInstanceDynamic)
  (if Valid
    (Rendering|Material|SetVectorParameterValue _overlaydynmat "BaseColor" (Math|Color|MakeColor 0.0 1.0 0.0) :!class /Script/Engine.MaterialInstanceDynamic)
    (else
      (Rendering|Material|SetVectorParameterValue _overlaydynmat "BaseColor" (Math|Color|MakeColor 1.0 0.0 0.0) :!class /Script/Engine.MaterialInstanceDynamic))))

(fn ClearValidationMat
  (Rendering|Material|SetScalarParameterValue (Variables|Default|GetOverlayDynMat) "Opacity" 0.0 :!class /Script/Engine.MaterialInstanceDynamic))