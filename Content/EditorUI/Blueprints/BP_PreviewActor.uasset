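; BP_PreviewActor is a placement preview actor that follows the cursor and signals whether a spot is valid.
; LocatePreview moves it to a Visibility trace hit under the cursor, while IsValidLocation requires its Collision to overlap no actors.
; SetPreviewValid tints Mesh green or red through the material Color parameter.
; SetUpPreview only stores and prints the class; the M_Validation dynamic material setup is unconnected.
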(event EventBeginPlay)

(event Collision|EventActorBeginOverlap
  (params (OtherActor :type Actor%20Object%20Reference)))

(event EventTick
  (params (DeltaSeconds :type Float%20%28single-precision%29)))

(fn ConstructionScript)

(fn SetPreviewValid
  (params (isValid :type Boolean))
  (if isValid
    (Rendering|Material|SetVectorParameterValueonMaterials (Variables|Default|GetMesh) "Color" (Math|Vector|MakeVector 0.0 1.0 0.0)) ; Verde
    (else
      (Rendering|Material|SetVectorParameterValueonMaterials (Variables|Default|GetMesh) "Color" (Math|Vector|MakeVector 1.0 0.0 0.0)) ; Rojo
    )))

(fn SetUpPreview
  (params (PreviewClass :type Actor%20Class%20Reference))
  (bind _output_get (Variables|Default|SetBlueprintClass PreviewClass))
  (Development|PrintString (Utilities|GetClassDisplayName _output_get)))

(fn IsValidLocation
  (return (Utilities|Array|IsEmpty (Collision|GetOverlappingActors (Variables|Default|GetCollision) 0 :!class /Script/Engine.PrimitiveComponent))))

(fn LocatePreview
  (bind _returnvalue (Game|GetPlayerController 0))
  (bind _hitresult (Game|Player|GetHitResultUnderCursorbyChannel _returnvalue "TraceTypeQuery1" true))
  (bind (_bblockinghit _binitialoverlap _time _distance _location) (Collision|BreakHitResult _hitresult))
  (Transformation|SetActorLocation _location _bblockinghit false))