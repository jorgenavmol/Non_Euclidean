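; BP_RecursivePurePortal is a portal actor that renders a recursive view and handles teleporting.
; Each tick, if ShouldUpdateRecursion passes, its PortalLogicComponent controls the recursions and renders the recursive view from recursion zero.
; It then runs viewport size and teleport checks every tick, regardless of that gate.
; BeginPlay and overlap events are disabled, and the construction script only calls the parent.
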(event EventBeginPlay
  (|CallParentFunction) ; This node is disabled and will not be called.\nDrag off pins to build functionality.
)

(event Collision|EventActorBeginOverlap
  (params (OtherActor :type Actor%20Object%20Reference))
  (|CallParentFunction OtherActor) ; This node is disabled and will not be called.\nDrag off pins to build functionality.
)

(event EventTick
  (params (DeltaSeconds :type Float%20%28single-precision%29))
  (bind _shouldupdate (CallFunction|ShouldUpdateRecursion))
  (if _shouldupdate
    (Class|PortalLogicComponent|ControlRecursions (Variables|Default|GetPortalLogicComponent))
    (Class|PortalLogicComponent|RenderRecursiveView (Variables|Default|GetPortalLogicComponent) "0, 0, 0" "0, 0, 0"))
  (CallFunction|CheckViewportSize)
  (CallFunction|ShouldTeleport))

(fn ConstructionScript
  (|CallParentFunction))