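; BP_ScalePortal is a portal variant that resizes the player on teleport.
; It extends the parent's TeleportPlayer by setting the player character's actor scale to that of the linked portal.
; ShouldUpdateRecursion passes when the portal lies within a cone around the camera's forward vector, tested by dot product, or the player overlaps the collision detector.
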(event EventBeginPlay
  (|CallParentFunction) ; This node is disabled and will not be called.\nDrag off pins to build functionality.
)

(event Collision|EventActorBeginOverlap
  (params (OtherActor :type Actor%20Object%20Reference))
  (|CallParentFunction OtherActor) ; This node is disabled and will not be called.\nDrag off pins to build functionality.
)

(event EventTick
  (params (DeltaSeconds :type Float%20%28single-precision%29))
  (|CallParentFunction DeltaSeconds) ; This node is disabled and will not be called.\nDrag off pins to build functionality.
)

(fn ConstructionScript
  (|CallParentFunction))

(fn TeleportPlayer
  (|CallParentFunction)
  (Transformation|SetActorScale3D (Game|GetPlayerCharacter 0) (Transformation|GetActorScale3D (Variables|Default|GetLinkedPortal))))

(fn ShouldUpdateRecursion
  (bind _returnvalue (Game|GetPlayerCameraManager 0))
  (return (or (> (Math|Vector|DotProduct (Math|Vector|Normalize (- (Transformation|GetActorLocation) (Camera|GetCameraLocation _returnvalue))) (Math|Vector|GetForwardVector (Camera|GetCameraRotation _returnvalue))) 0.6) (Collision|IsOverlappingActor (Variables|Default|GetCollisionDetector) (Game|GetPlayerCharacter 0) :!class /Script/Engine.PrimitiveComponent))))