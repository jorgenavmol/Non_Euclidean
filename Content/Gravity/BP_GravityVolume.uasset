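; BP_GravityVolume is a volume that changes the gravity direction of actors entering its collision if they implement BPI_GravityReceiver.
; On begin overlap it records the actor and sends its normalized GravityDirection, with itself as the gravity zone, through an interface message.
; On end overlap it removes the actor and sends the player character's OriginalGravityDirection, whichever actor left.
; A loop re-sending gravity to tracked actors is disconnected and never runs.
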(event OnComponentEndOverlap(Collision)
  (params (OverlappedComponent :type Primitive%20Component%20Object%20Reference) (OtherActor :type Actor%20Object%20Reference) (OtherComp :type Primitive%20Component%20Object%20Reference) (OtherBodyIndex :type Integer))
  (if (Utilities|DoesObjectImplementInterface OtherActor "/Game/Gravity/BPI_GravityReceiver.BPI_GravityReceiver_C")
    (Utilities|Array|RemoveItem (Variables|Default|GetOverlappingActors) OtherActor)
    (Class|BPIGravityReceiver|SetCustomGravityDirection(Message) OtherActor (Variables|/Game/FirstPerson/Blueprints/BP_FirstPersonCharacter.BP_FirstPersonCharacter_C|GetOriginalGravityDirection (.AsBP%20First%20Person%20Character (Utilities|Casting|CastToBP_FirstPersonCharacter (Game|GetPlayerCharacter 0)))) (Components|GetOwner OverlappedComponent))))

(event OnComponentBeginOverlap(Collision)
  (params (OverlappedComponent :type Primitive%20Component%20Object%20Reference) (OtherActor :type Actor%20Object%20Reference) (OtherComp :type Primitive%20Component%20Object%20Reference) (OtherBodyIndex :type Integer) (bFromSweep :type Boolean) (SweepResult :type Hit%20Result%20Structure%20%28by%20ref%29))
  (if (Utilities|DoesObjectImplementInterface OtherActor "/Game/Gravity/BPI_GravityReceiver.BPI_GravityReceiver_C")
    (Development|PrintString "Hello")
    (Utilities|Array|Add (Variables|Default|GetOverlappingActors) OtherActor)
    (Class|BPIGravityReceiver|SetCustomGravityDirection(Message) OtherActor (Math|Vector|Normalize (Variables|Default|GetGravityDirection)) (Components|GetOwner OverlappedComponent))))

(event EventBeginPlay)

(event EventTick
  (params (DeltaSeconds :type Float%20%28single-precision%29)))

(fn ConstructionScript)