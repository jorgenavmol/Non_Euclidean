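; BP_WarpedCorridor is a corridor structure that contains two portals linked to each other.
; Its Construction Script casts the Portal1 and Portal2 child actors to BP_Portal and sets each one as the other's LinkedPortal, so the pair is connected at construction.
; The event graph has no active logic; a node enabling collision on the Top, Left and Right components is left unconnected.
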(event EventBeginPlay)

(event Collision|EventActorBeginOverlap
  (params (OtherActor :type Actor%20Object%20Reference)))

(event EventTick
  (params (DeltaSeconds :type Float%20%28single-precision%29)))

(fn ConstructionScript
  (|CallParentFunction)
  (bind _asbp_portal (Utilities|Casting|CastToBP_Portal (Variables|/Script/Engine.ChildActorComponent|GetChildActor (Variables|Default|GetPortal1))))
  (bind _asbp_portal_2 (Utilities|Casting|CastToBP_Portal (Variables|/Script/Engine.ChildActorComponent|GetChildActor (Variables|Default|GetPortal2))))
  (Variables|/Game/PortalSystem/BP_Portal.BP_Portal_C|SetLinkedPortal _asbp_portal _asbp_portal_2)
  (Variables|/Game/PortalSystem/BP_Portal.BP_Portal_C|SetLinkedPortal _asbp_portal_2 _asbp_portal))