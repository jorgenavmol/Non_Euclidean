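; BP_GravWall is a wall structure that carries its own gravity zone, pulling along the wall's negative right axis.
; Its construction script casts the GravZone child actor to BP_GravityVolume and derives that volume's GravityDirection from the Wall component's world rotation.
; On BeginPlay, Wall gets query and physics collision while VisualMesh has collision disabled, separating the collision surface from the visual.
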(event EventBeginPlay
  (Collision|SetCollisionEnabled (Variables|Default|GetWall) "QueryAndPhysics")
  (Collision|SetCollisionEnabled (Variables|Default|GetVisualMesh) "NoCollision"))

(event Collision|EventActorBeginOverlap
  (params (OtherActor :type Actor%20Object%20Reference)))

(event EventTick
  (params (DeltaSeconds :type Float%20%28single-precision%29)))

(fn ConstructionScript
  (|CallParentFunction)
  (bind _asbp_gravity_volume (Utilities|Casting|CastToBP_GravityVolume (Variables|/Script/Engine.ChildActorComponent|GetChildActor (Variables|Default|GetGravZone))))
  (Variables|/Game/Gravity/BP_GravityVolume.BP_GravityVolume_C|SetGravityDirection _asbp_gravity_volume (Math|Vector|NegateVector (Math|Vector|GetRightVector (Transformation|GetWorldRotation (Variables|Default|GetWall))))))